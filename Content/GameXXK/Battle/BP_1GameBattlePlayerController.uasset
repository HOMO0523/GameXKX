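; Battle player controller that drives level and chapter progression through a map selection widget (UI_地图选择), shown in UI-only input mode on BeginPlay.
; Starting a level stores the Boss flag and map info, but every level-type branch is an empty placeholder, so it auto-completes after a short delay.
; Normal completion advances the level index and reopens the map.
; Boss completion removes the map, creating the next chapter's until the chapter cap.
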(event `self.ReceiveBeginPlay`
  ;[1 1 1] 进入游戏
  (bind _returnvalue (`|CreateWidget` "/Game/1Game/UI/UI_地图选择.UI_地图选择_C"))
  (`UserWidget.AddToViewport` _returnvalue 200)
  (bind _output_get (set `self.UI_地图选择` _returnvalue))
  (`WidgetBlueprintLibrary.SetInputMode_UIOnlyEx` self _output_get))

(event `Ev_结束当前关卡`
  (bind `_ui_地图选择` (`self.UI_地图选择`))
  (bind `_ui_地图选择_2` (`self.UI_地图选择`))
  ;[1 1 1] 结束当前关卡,获得奖励
  (if (`self.Boss`)
    ;;[1 1 1] 创建新的地图
    (`Widget.RemoveFromParent` (`self.UI_地图选择`))
    (if (not (>= (`self.当前章节序号`) 3))
      (set `self.当前关卡序号` 0)
      (`/Engine/EditorBlueprintResources/StandardMacros.IncrementInt` (`self.当前章节序号`)
        (:`  `
          (bind _returnvalue (`|CreateWidget` "/Game/1Game/UI/UI_地图选择.UI_地图选择_C" :!label _label))
          (`UserWidget.AddToViewport` _returnvalue 200)
          (set `self.UI_地图选择` _returnvalue))))
    (else
      (`/Engine/EditorBlueprintResources/StandardMacros.IncrementInt` (`self.当前关卡序号`)
        (:`  `
          (`self.UI_地图选择`
            (:`then`
              (`Widget.SetVisibility` `_ui_地图选择_2` "SelfHitTestInvisible")
              (`Widget.SetRenderOpacity` `_ui_地图选择_2` 0.0)
              (`KismetSystemLibrary.Delay` 0.2)
              (`Widget.SetRenderOpacity` `_ui_地图选择` 1.0)
              (`/Game/1Game/UI/UI_地图选择.Ev_重新打开地图` `_ui_地图选择` (`self.当前关卡序号`)))
            (:`else`
              (goto _label))))))))

(event `Ev_开始新的关卡`
  (params (Boss :type Boolean) (`ST_地图选择信息` :type "/Game/1Game/Data/ST_地图选择信息 Structure (by ref)"))
  ;[1 1 1] 开始新的关卡
  (set `self.Boss` Boss)
  (set `self.当前地图的信息结构` `ST_地图选择信息`)
  (switch `/Game/1Game/Data/E_地图关卡类型` (`.地图关卡类型_22_711E8CF347CA6BC59877728CAD8F3642` (break `/Game/1Game/Data/ST_地图选择信息` (`self.当前地图的信息结构`)))
    (:`NewEnumerator0`
      _)
    (:`NewEnumerator1`
      _)
    (:`NewEnumerator2`
      _)
    (:`NewEnumerator3`
      _)
    (:`NewEnumerator4`
      _)
    (:`NewEnumerator5`
      _))
  (`KismetSystemLibrary.Delay` 1.0)
  (`self.Ev_结束当前关卡`))

(fn `UserConstructionScript`)